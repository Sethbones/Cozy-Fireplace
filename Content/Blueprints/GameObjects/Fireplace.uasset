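; Fireplace game object that the player fuels with collected wood to light its fire.
; On GeneralInteraction it checks the Globals game instance and, if not yet full and WoodCount meets WoodRequirement, zeroes the wood, sets FirePlaceFull and shows the PFire component.
; Disconnected leftover nodes would double the requirement, increment DayNumber and reload the level, but never run.
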(event `/Game/Blueprints/misc/GlobalClassFunctionCalls.General_Interaction`
  (params (CurrentActor :type "Actor Object Reference"))
  (bind _asglobals (cast `/Game/Blueprints/Globals` (`GameplayStatics.GetGameInstance`)))
  (if (!= (`/Game/Blueprints/Globals.FirePlaceFull` _asglobals) true)
    (if (>= (`/Game/Blueprints/Globals.WoodCount` _asglobals) (`/Game/Blueprints/Globals.WoodRequirement` _asglobals))
      (set `/Game/Blueprints/Globals.WoodCount` 0 _asglobals)
      (set `/Game/Blueprints/Globals.FirePlaceFull` true _asglobals)
      (`SceneComponent.SetVisibility` (`self.P_Fire`) true false))))

(fn `UserConstructionScript`)