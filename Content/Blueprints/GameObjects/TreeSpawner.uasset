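; Spawner actor that keeps adding Tree actors at random positions derived from its own location, until its tracked array exceeds MaxTreeSpawn.
; Tick checks the array length, then a Delay paces each spawn.
; X and Y add a random offset to the actor's location, then multiply that whole sum by actor scale; Z stays unchanged.
; Each tree joins TreeArray and receives a SpawnedFrom reference to the spawner.
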(event `self.ReceiveTick`
  (params (DeltaSeconds :type "Float (single-precision)"))
  (bind (_returnvalue_x _returnvalue_y) (`KismetMathLibrary.BreakVector` (`self.K2_GetActorLocation`)))
  (bind _returnvalue (`self.GetTransform`))
  (bind (_returnvalue_x_2 _returnvalue_y_2 _returnvalue_z) (`KismetMathLibrary.BreakVector` (`self.K2_GetActorLocation`)))
  (bind _positiverange (`self.PositiveRange`))
  (bind _negativerange (`self.NegativeRange`))
  ;[1 1 1] Spawns trees in a range, used arrows as position markers for spawning
  (`|ExecutionSequence`
    (:`then_1`
      (if (<= (`KismetArrayLibrary.Array_Length` (`self.TreeArray`)) (`self.MaxTreeSpawn`))
        (`KismetSystemLibrary.Delay` (`self.SpawnDelay`))
        (bind _returnvalue_2 (`|SpawnActorFromClass` "/Game/Blueprints/GameObjects/Tree.Tree_C" (`KismetMathLibrary.MakeTransform` (`KismetMathLibrary.MakeVector` (* (+ (`KismetMathLibrary.RandomFloatInRange` _negativerange _positiverange) _returnvalue_x) (.x (.scale _returnvalue))) (* (+ _returnvalue_y (`KismetMathLibrary.RandomFloatInRange` _negativerange _positiverange)) (.y (.scale _returnvalue))) _returnvalue_z)) "Undefined" "OverrideRootScale" null null))
        (`KismetArrayLibrary.Array_Add` (`self.TreeArray`) _returnvalue_2)
        (set `/Game/Blueprints/GameObjects/Tree.SpawnedFrom` self _returnvalue_2)))))

(fn `UserConstructionScript`)