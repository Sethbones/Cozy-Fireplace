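; Bed actor the player interacts with to sleep and advance to the next day.
; On GeneralInteraction it acts only if the Globals game instance reports the fireplace full.
; It then scales the wood requirement by the day multiplier, increments the day, clears fireplace, tutorial and wood count state, and reloads FirstPersonMap.
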(event `self.ReceiveTick`
  (params (DeltaSeconds :type "Float (single-precision)")))

(event `/Game/Blueprints/misc/GlobalClassFunctionCalls.General_Interaction`
  (params (CurrentActor :type "Actor Object Reference"))
  (bind _asglobals (cast `/Game/Blueprints/Globals` (`GameplayStatics.GetGameInstance`)))
  (if (`/Game/Blueprints/Globals.FirePlaceFull` _asglobals)
    (set `/Game/Blueprints/Globals.WoodRequirement` (`KismetMathLibrary.Round` (* (`/Game/Blueprints/Globals.WoodRequirement` _asglobals) (`/Game/Blueprints/Globals.DayTreeCountMultiplier` _asglobals))) _asglobals)
    (bind _output_get (set `/Game/Blueprints/Globals.DayNumber` (+ (`/Game/Blueprints/Globals.DayNumber` _asglobals) 1) _asglobals))
    (set `/Game/Blueprints/Globals.FirePlaceFull` false _asglobals)
    (set `/Game/Blueprints/Globals.inTutorial` false _asglobals)
    (set `/Game/Blueprints/Globals.WoodCount` 0 _asglobals)
    (`GameplayStatics.OpenLevelBySoftObjectPtr` "/Game/FirstPerson/Maps/FirstPersonMap.FirstPersonMap")))

(fn `UserConstructionScript`)