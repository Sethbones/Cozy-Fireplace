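; Interactable door actor that swings open or closed each time GeneralInteraction is called.
; Separate open and close timelines drive the yaw of the Cylinder component's relative rotation.
; DoorClosed and DoorOpened flags are cleared during motion and set on completion, so interactions mid-swing are ignored.
; The open sound plays as opening starts, while the close sound plays once closing finishes.
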(event `/Game/Blueprints/misc/GlobalClassFunctionCalls.General_Interaction`
  (params (CurrentActor :type "Actor Object Reference"))
  (bind _returnvalue (`self.K2_GetActorLocation`))
  (if (`self.DoorClosed`)
    (`GameplayStatics.PlaySoundAtLocation` "/Game/Sounds/DoorOpen.DoorOpen" _returnvalue (struct) 1.0 1.0 0.0 null null null null)
    (bind (_direction _newtrack_0) (`Timeline|Door Open` :!via `PlayFromStart`)
      (:`Update`
        (`SceneComponent.K2_SetRelativeRotation` (`self.Cylinder`) (`KismetMathLibrary.MakeRotator` 0.0 0.0 _newtrack_0) false false)
        (set `self.DoorClosed` false))
      (:`Finished`
        (set `self.DoorOpened` true)))
    (elif (`self.DoorOpened`)
      (bind (_direction_2 _newtrack_0_2) (`Timeline|DoorClose` :!via `PlayFromStart`)
        (:`Update`
          (`SceneComponent.K2_SetRelativeRotation` (`self.Cylinder`) (`KismetMathLibrary.MakeRotator` 0.0 0.0 _newtrack_0_2) false false)
          (set `self.DoorOpened` false))
        (:`Finished`
          (set `self.DoorClosed` true)
          (`GameplayStatics.PlaySoundAtLocation` "/Game/Sounds/DoorClose.DoorClose" _returnvalue (struct) 1.0 1.0 0.0 null null null null))))))

(fn `UserConstructionScript`)