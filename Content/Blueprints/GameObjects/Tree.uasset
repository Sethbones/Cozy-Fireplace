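; Choppable tree actor that sprouts, dries out and withers through timeline-driven stages, then leaves a FallenLog if left standing.
; Tick eases the tree toward its actor height, plays a bump timeline when health changes and tints the trunk at low health.
; Chopping warms the player and briefly pauses the current stage timeline.
; OnDeath adds stage-dependent random wood to Globals, and destruction removes the tree from its TreeSpawner.
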(event `self.ReceiveBeginPlay`
  (`|ExecutionSequence`
    (:`then_0`
      (set `self.HealthWatcher` (`self.TreeHealth`)))
    (:`then_1`
      (while (`self.StartGrowAndDecay`)
        _)
      (set `self.treeState` 0)
      (bind (_direction _newtrack_0) (`Timeline|LeavesSprout` :!via `PlayFromStart`)
        (:`Update`
          (`SceneComponent.SetWorldScale3D` (`self.Cone`) (`KismetMathLibrary.Conv_DoubleToVector` _newtrack_0)))
        (:`Finished`
          (set `self.treeState` 1)
          (bind (_direction_2 _newtrack_1) (`Timeline|LeavesDrought` :!via `PlayFromStart`)
            (:`Update`
              (for _array_element (`|MakeArray` (`self.Cone`) (`self.Cone1`) (`self.Cone2`))
                (`MeshComponent.SetVectorParameterValueOnMaterials` _array_element "Param" _newtrack_1)))
            (:`Finished`
              (set `self.treeState` 2)
              (for _array_element_2 (`|MakeArray` (`self.Cone`) (`self.Cone1`) (`self.Cone2`))
                (`SceneComponent.SetWorldScale3D` _array_element_2 (0.0 0.0 0.0))
                (`SceneComponent.SetWorldScale3D` (`self.TreeContainer`) (1.0 1.0 0.5)))
              (`KismetSystemLibrary.Delay` 6.0)
              (`|SpawnActorFromClass` "/Game/Blueprints/GameObjects/FallenLog.FallenLog_C" (`self.GetTransform`) "Undefined" "OverrideRootScale" null null)
              (`self.K2_DestroyActor`))))))))

(event `self.ReceiveTick`
  (params (DeltaSeconds :type "Float (single-precision)"))
  (bind _treecontainer (`self.TreeContainer`))
  (bind (_returnvalue_x _returnvalue_y _returnvalue_z) (`KismetMathLibrary.BreakVector` (`SceneComponent.K2_GetComponentLocation` _treecontainer)))
  (`|ExecutionSequence`
    (:`then_0`
      (if (!= (`self.HealthWatcher`) (`self.TreeHealth`))
        (`|ExecutionSequence`
          (:`then_0`
            (bind _output_get (set `self.HealthWatcher` (`self.TreeHealth`)))
            (`KismetSystemLibrary.PrintString` (`KismetStringLibrary.Conv_IntToString` _output_get)))
          (:`then_1`
            (bind (_direction _newtrack_1) (`Timeline|Timeline` :!via `PlayFromStart`)
              (:`Update`
                (`SceneComponent.K2_SetWorldLocation` _treecontainer (`KismetMathLibrary.MakeVector` _returnvalue_x _returnvalue_y (+ _returnvalue_z _newtrack_1)) false false)))))))
    (:`then_1`
      (if (== (`self.TreeHealth`) 1)
        (`MeshComponent.SetVectorParameterValueOnMaterials` (`self.Cylinder`) "Param" (1.0 1.0 0.0))
        (elif (== (`self.TreeHealth`) 0)
          (`MeshComponent.SetVectorParameterValueOnMaterials` (`self.Cylinder`) "Param" (1.0 0.0 0.0)))))
    (:`then_2`
      (`self.TreeRaise`))))

(event `onChop`
  (bind _leavessprout (`self.LeavesSprout`))
  (bind _leavesdrought (`self.LeavesDrought`))
  (bind _asbp_first_person_character (cast `/Game/FirstPerson/Blueprints/BP_FirstPersonCharacter` (`GameplayStatics.GetPlayerCharacter` 0)))
  (set `/Game/FirstPerson/Blueprints/BP_FirstPersonCharacter.Temperature` (+ (`/Game/FirstPerson/Blueprints/BP_FirstPersonCharacter.Temperature` _asbp_first_person_character) 1.0) _asbp_first_person_character)
  (`KismetSystemLibrary.PrintString` (`KismetStringLibrary.Concat_StrStr` "hitting a tree in state: " (`KismetStringLibrary.Conv_IntToString` (`self.treeState`))))
  ;[1 1 1] Game Feel Galore
  (`GameplayStatics.PlaySound2D` "/Game/Sounds/TreeHit.TreeHit" 1.0 1.0 0.0 null null)
  (`|ExecutionSequence`
    (:`then_0`
      (if (== (`self.treeState`) 0)
        (`|ExecutionSequence`
          (:`then_0`
            (bind _pausepoint (`/Game/Blueprints/misc/Whythefucks.Pause Timeline` _leavessprout)))
          (:`then_1`
            (`KismetSystemLibrary.RetriggerableDelay` 1.0)
            (`/Game/Blueprints/misc/Whythefucks.Resume Timeline` _leavessprout _pausepoint)))))
    (:`then_1`
      (if (== (`self.treeState`) 1)
        (`|ExecutionSequence`
          (:`then_0`
            (bind _pausepoint_2 (`/Game/Blueprints/misc/Whythefucks.Pause Timeline` _leavesdrought)))
          (:`then_1`
            (`KismetSystemLibrary.RetriggerableDelay` 1.0)
            (`/Game/Blueprints/misc/Whythefucks.Resume Timeline` _leavesdrought _pausepoint_2)))))))

(event `self.ReceiveDestroyed`
  (bind _astree_spawner (cast `/Game/Blueprints/GameObjects/TreeSpawner` (`self.SpawnedFrom`)))
  (bind _returnvalue (`KismetArrayLibrary.Array_RemoveItem` (`/Game/Blueprints/GameObjects/TreeSpawner.TreeArray` _astree_spawner) self))
  (if _returnvalue
    _))

(fn `onDeath`
  (bind _asglobals (cast `/Game/Blueprints/Globals` (`GameplayStatics.GetGameInstance`)))
  (`GameplayStatics.PlaySound2D` "/Game/Sounds/TreeFall.TreeFall" 1.0 1.0 0.0 null null)
  (if (== (`self.treeState`) 0)
    (set `/Game/Blueprints/Globals.WoodCount` (+ (`KismetMathLibrary.RandomIntegerInRange` 1 3) (`/Game/Blueprints/Globals.WoodCount` _asglobals)) _asglobals)
    (`self.K2_DestroyActor`)
    (elif (== (`self.treeState`) 1)
      (set `/Game/Blueprints/Globals.WoodCount` (+ (`KismetMathLibrary.RandomIntegerInRange` 4 6) (`/Game/Blueprints/Globals.WoodCount` _asglobals)) _asglobals)
      (`self.K2_DestroyActor`)
      (elif (== (`self.treeState`) 2)
        (set `/Game/Blueprints/Globals.WoodCount` (+ (`KismetMathLibrary.RandomIntegerInRange` 1 2) (`/Game/Blueprints/Globals.WoodCount` _asglobals)) _asglobals)
        (`self.K2_DestroyActor`)))))

(fn `TreeRaise`
  (bind (_returnvalue_x _returnvalue_y _returnvalue_z) (`KismetMathLibrary.BreakVector` (`self.K2_GetActorLocation`)))
  (bind _treecontainer (`self.TreeContainer`))
  (bind (_returnvalue_x_2 _returnvalue_y_2 _returnvalue_z_2) (`KismetMathLibrary.BreakVector` (`SceneComponent.K2_GetComponentLocation` _treecontainer)))
  (`SceneComponent.K2_SetWorldLocation` _treecontainer (`KismetMathLibrary.MakeVector` _returnvalue_x_2 _returnvalue_y_2 (`KismetMathLibrary.Lerp` _returnvalue_z_2 _returnvalue_z 0.5)) false false)
  (`/Engine/EditorBlueprintResources/StandardMacros.IsValid` _treecontainer
    (:`Is Valid`
      (if (== (`KismetMathLibrary.Round` _returnvalue_z_2) 530)
        (set `self.StartGrowAndDecay` true)
        (return)))))

(fn `UserConstructionScript`)