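; Note is an interactable world object that opens the Diary widget and appears only on day 10.
; Shortly after BeginPlay it reads DayNumber from the Globals game instance and hides itself on any other day.
; On GeneralInteraction it stops the LevelMusic audio, adds a new Diary widget to the viewport and switches input to UI only.
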(event `self.ReceiveBeginPlay`
  (`KismetSystemLibrary.Delay` 0.2)
  (bind _asglobals (cast `/Game/Blueprints/Globals` (`GameplayStatics.GetGameInstance`)))
  (if (== 10 (`/Game/Blueprints/Globals.DayNumber` _asglobals))
    (`self.SetActorHiddenInGame` false)
    (else
      (`self.SetActorHiddenInGame` true))))

(event `self.ReceiveTick`
  (params (DeltaSeconds :type "Float (single-precision)")))

(event `/Game/Blueprints/misc/GlobalClassFunctionCalls.General_Interaction`
  (params (CurrentActor :type "Actor Object Reference"))
  (bind _returnvalue (`GameplayStatics.GetPlayerController` 0))
  (bind _returnvalue_2 (`GameplayStatics.GetActorOfClass` "/Game/Blueprints/misc/LevelMusic.LevelMusic_C"))
  (`/Engine/EditorBlueprintResources/StandardMacros.IsValid` _returnvalue_2
    (:`Is Valid`
      (`AudioComponent.Stop` (`/Game/Blueprints/misc/LevelMusic.Audio` _returnvalue_2)))
    (:`Is Not Valid`
      _))
  (bind _returnvalue_3 (`|CreateWidget` "/Game/Blueprints/UI/Diary.Diary_C" _returnvalue))
  (`UserWidget.AddToViewport` _returnvalue_3 0)
  (`WidgetBlueprintLibrary.SetInputMode_UIOnlyEx` _returnvalue null))

(fn `UserConstructionScript`)