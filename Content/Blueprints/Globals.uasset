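; Globals Blueprint that holds shared routines for the game's ending and for a timed screen shake.
; StartEnding runs once via the InEnding flag, replacing all widgets with the Ending widget, switching to UI-only input with a cursor and stopping level music.
; StartScreenShake stores an epicenter and triggers the ScreenShake event, which plays the Ragolo sound and repeats the EndingShake world camera shake three times, spaced by delays.
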(event `ScreenShake`
  (bind _screenshakevector (`self.ScreenShakeVector`))
  (`GameplayStatics.PlaySound2D` "/Game/Blueprints/Ragolo.Ragolo" 1.0 1.0 0.0 null null)
  (`GameplayStatics.PlayWorldCameraShake` "/Game/Blueprints/misc/EndingShake.EndingShake_C" _screenshakevector 0.0 500.0)
  (`KismetSystemLibrary.Delay` 2.0)
  (`GameplayStatics.PlayWorldCameraShake` "/Game/Blueprints/misc/EndingShake.EndingShake_C" _screenshakevector 0.0 500.0)
  (`KismetSystemLibrary.Delay` 2.0)
  (`GameplayStatics.PlayWorldCameraShake` "/Game/Blueprints/misc/EndingShake.EndingShake_C" _screenshakevector 0.0 500.0))

(fn `StartEnding`
  (if (not (`self.InEnding`))
    (`WidgetLayoutLibrary.RemoveAllWidgets`)
    (bind _returnvalue (`|CreateWidget` "/Game/Blueprints/UI/Ending.Ending_C"))
    (`UserWidget.AddToViewport` _returnvalue 0)
    (`WidgetBlueprintLibrary.SetInputMode_UIOnlyEx` (`GameplayStatics.GetPlayerController` 0) null)
    (set `self.InEnding` true)
    (set `PlayerController.bShowMouseCursor` true (`GameplayStatics.GetPlayerController` 0))
    (bind _returnvalue_2 (`GameplayStatics.GetActorOfClass` "/Game/Blueprints/misc/LevelMusic.LevelMusic_C"))
    (`/Engine/EditorBlueprintResources/StandardMacros.IsValid` _returnvalue_2
      (:`Is Valid`
        (`AudioComponent.Stop` (`/Game/Blueprints/misc/LevelMusic.Audio` _returnvalue_2))))))

(fn `StartScreenShake`
  (params (`Actor Transform` :type "Vector Structure"))
  (set `self.ScreenShakeVector` `Actor Transform`)
  (`self.ScreenShake`))